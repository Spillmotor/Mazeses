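; BP_SlidingDoor_Y is a sliding door that moves itself on a timed sequence from BeginPlay, with no player trigger.
; After a short delay, it caches its location and Timeline_0 applies a vector offset to the actor without sweeping.
; Timeline_0's Update also feeds a longer Delay, which then re-caches the location and starts Timeline_1 to apply a second offset from there.
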(event `self.ReceiveBeginPlay`
  (`KismetSystemLibrary.Delay` 3.0)
  (set `self.Initaial Location` (`self.K2_GetActorLocation`))
  (bind (_direction _movement) (`Timeline|Timeline_0` :!via `PlayFromStart`)
    (:`Update`
      (`self.K2_SetActorLocation` (+ (`self.Initaial Location`) _movement))
      (`KismetSystemLibrary.Delay` 6.0)
      (set `self.Initaial Location` (`self.K2_GetActorLocation`))
      (bind (_direction_2 _movement_2) (`Timeline|Timeline_1` :!via `PlayFromStart`)
        (:`Update`
          (`self.K2_SetActorLocation` (+ (`self.Initaial Location`) _movement_2)))))))

(fn `UserConstructionScript`)