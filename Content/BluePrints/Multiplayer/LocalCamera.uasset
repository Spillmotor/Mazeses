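; LocalCamera is a shared local-multiplayer camera that frames four player characters by tracking their midpoint and zooming with their spread.
; Each tick it moves a Box to the average of the four positions and eases the spring arm length toward a clamped, offset distance value.
; That distance is the larger of only the player 1–2 and 3–4 separations, so other pairings do not affect zoom.
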(event `self.ReceiveBeginPlay`
  ;[1 1 1] Move camera in characters index
  (`|ExecutionSequence`
    (:`then_0`
      (set `self.C1` (`GameplayStatics.GetPlayerCharacter` 0))
      (set `self.C2` (`GameplayStatics.GetPlayerCharacter` 1))
      (set `self.C3` (`GameplayStatics.GetPlayerCharacter` 2))
      (set `self.C4` (`GameplayStatics.GetPlayerCharacter` 3)))
    (:`then_1`
      (set `self.CameraYPosition` (.y (`SceneComponent.K2_GetComponentLocation` (`self.SpringArm`))))
      (set `self.CameraXPosition` (.x (`SceneComponent.K2_GetComponentLocation` (`self.SpringArm`))))
      (set `self.CamerastartPosition` (`KismetMathLibrary.MakeVector` 0.0 0.0 (.z (`self.K2_GetActorLocation`)))))))

(event `Set longest Disnatnce between players`
  (bind _c4 (`self.C4`))
  (bind _c3 (`self.C3`))
  (bind _c2 (`self.C2`))
  (bind _c1 (`self.C1`))
  ;[1 1 1] Make longest distane of 2 players
  (set `self.Longest Distance` (- (`.MaxValue` (`KismetMathLibrary.MaxOfFloatArray` (`|MakeArray` (`self.GetDistanceTo` _c1 _c2) (`self.GetDistanceTo` _c4 _c3) (`self.GetDistanceTo` _c3 _c4) (`self.GetDistanceTo` _c2 _c1)))) 1300.0)))

(event `Set center point`
  ;[1 1 1] Set center point between players
  (set `self.CenterPosition` (/ (+ (`self.K2_GetActorLocation` (`self.C1`)) (`self.K2_GetActorLocation` (`self.C2`)) (`self.K2_GetActorLocation` (`self.C3`)) (`self.K2_GetActorLocation` (`self.C4`))) (4.0 4.0 4.0))))

(event `self.ReceiveTick`
  (params (DeltaSeconds :type "Float (single-precision)"))
  ;[1 1 1] Activate events made.
  (set `self.Delta` DeltaSeconds)
  (`|ExecutionSequence`
    (:`then_0`
      (`self.Set longest Disnatnce between players`)
      (`self.Set center point`)
      (`self.Camera zoom`)
      (`self.Set Box Position`))))

(event `Set Box Position`
  ;[1 1 1] Set box position
  (`SceneComponent.K2_SetWorldLocation` (`self.Box`) (`self.CenterPosition`) false false))

(event `Camera zoom`
  (bind _springarm (`self.SpringArm`))
  ;[1 1 1] Camera zoom. kan endre på min max og speed.
  (set `SpringArmComponent.TargetArmLength` (`KismetMathLibrary.FInterpTo` (`SpringArmComponent.TargetArmLength` _springarm) (`KismetMathLibrary.FMax` (`KismetMathLibrary.FMin` (`self.Longest Distance`) 800.0) 200.0) (`self.Delta`) 0.5) _springarm))

(fn `UserConstructionScript`)